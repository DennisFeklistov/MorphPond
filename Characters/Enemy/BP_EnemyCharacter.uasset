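; Enemy character that targets the player, with AI events for bite, jump, landing and a tongue or cannonball special attack.
; HurtBox overlaps from player bites and attack actors trigger WeakAttack: knockback, blood, flash, hitstop, damage and a scale-blip timeline during temporary invincibility.
; At zero health, Death plays effects and hitstop, credits the killer, then destroys the enemy, passing any special ability to the player.
; Several disconnected older hit and collision chains remain.
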(event OnComponentBeginOverlap(HurtBox)
  (params (OverlappedComponent :type Primitive%20Component%20Object%20Reference) (OtherActor :type Actor%20Object%20Reference) (OtherComp :type Primitive%20Component%20Object%20Reference) (OtherBodyIndex :type Integer) (bFromSweep :type Boolean) (SweepResult :type Hit%20Result%20Structure%20%28by%20ref%29))
  ;[1 1 1] Hit by Attack (clean up)
  (bind _asbp_player_character (Utilities|Casting|CastToBP_PlayerCharacter OtherActor)
    (:then
      (bind _output_get (Variables|Default|SetAttacker _asbp_player_character))
      (if (Math|Boolean|ANDBoolean (Variables|/Game/MorphPond/Characters/BP_CharacterBaseClass.BP_CharacterBaseClass_C|GetIsBiting? _asbp_player_character) (not (Variables|Default|GetInvincibleToWeakAttacks)) (Components|ComponentHasTag OtherComp "Bite"))
        (bind _output_get_2 (Variables|Default|SetIncomingDamage (Variables|/Game/MorphPond/Characters/BP_CharacterBaseClass.BP_CharacterBaseClass_C|GetBiteDamage _output_get)))
        (CallFunction|WeakAttack (Variables|Default|GetAttacker) 1.0 _output_get_2)))
    (:CastFailed
      (bind _asbp_3dattack_base_class (Utilities|Casting|CastToBP_3DAttackBaseClass OtherActor)
        (:then
          (bind _asbp_player_character_2 (Utilities|Casting|CastToBP_PlayerCharacter (Variables|/Script/Engine.Actor|GetInstigator _asbp_3dattack_base_class)))
          (Variables|Default|SetAttacker _asbp_player_character_2)
          (Utilities|IsValid _asbp_player_character_2
            (:Is%20Valid
              (if (and (Variables|/Game/MorphPond/Characters/BP_CharacterBaseClass.BP_CharacterBaseClass_C|GetIsSpecialAttacking? _asbp_player_character_2) (not (Variables|Default|GetInvincibleToWeakAttacks)))
                (Variables|Default|SetIncomingDamage (Variables|/Game/MorphPond/Attacks/BP_3DAttackBaseClass.BP_3DAttackBaseClass_C|GetDamage _asbp_3dattack_base_class))
                (CallFunction|WeakAttack (Variables|Default|GetAttacker) 1.0 (Variables|Default|GetIncomingDamage) :!label _label)))))
        (:CastFailed
          (bind _asbp_2dattack_base_class (Utilities|Casting|CastToBP_2DAttackBaseClass OtherActor))
          (bind _asbp_player_character_3 (Utilities|Casting|CastToBP_PlayerCharacter (Variables|/Script/Engine.Actor|GetInstigator _asbp_2dattack_base_class)))
          (Variables|Default|SetAttacker _asbp_player_character_3)
          (Utilities|IsValid _asbp_player_character_3
            (:Is%20Valid
              (if (and (Variables|/Game/MorphPond/Characters/BP_CharacterBaseClass.BP_CharacterBaseClass_C|GetIsBiting? _asbp_player_character_3) (not (Variables|Default|GetInvincibleToWeakAttacks)))
                (bind _asbp_fangs (Utilities|Casting|CastToBP_Fangs OtherActor))
                (Variables|Default|SetIncomingDamage (Variables|/Game/MorphPond/Attacks/BP_2DAttackBaseClass.BP_2DAttackBaseClass_C|GetDamage _asbp_fangs))
                (goto _label)))))))))

(event OnComponentBeginOverlap(Sphere_0)
  (params (OverlappedComponent :type Primitive%20Component%20Object%20Reference) (OtherActor :type Actor%20Object%20Reference) (OtherComp :type Primitive%20Component%20Object%20Reference) (OtherBodyIndex :type Integer) (bFromSweep :type Boolean) (SweepResult :type Hit%20Result%20Structure%20%28by%20ref%29)))

(event Custom|AI%20Attack
  ;[1 1 1] Bite Attack
  (CallFunction|BiteAttackAction))

(event Custom|AI%20Jump
  ;[1 1 1] JumpAnim
  (CallFunction|JumpAction))

(event Custom|ResumeParticles
  ;[1 1 1] Particle Hitstop
  (Class|NiagaraComponent|SetPaused (Variables|Default|GetTarget%20Particle) false))

(event Custom|Weak%20Attack
  (params (Originator :type Actor%20Object%20Reference) (Knockback%20Multiplier :type Float%20%28double-precision%29) (Damage :type Integer))
  (bind _visiblebody (Variables|Default|GetVisibleBody))
  (bind _fmod_hitbyplayerbite (Variables|Default|GetFMOD_HitByPlayerBite))
  ;[1 1 1] Hit by Weak Attack
  (Variables|Default|SetInvincibleToWeakAttacks true)
  (Camera|PlayWorldCameraShake "/Game/MorphPond/Camera/ScreenShake_Large.ScreenShake_Large_C" (Transformation|GetActorLocation) 0.0 5e+03 1.0 true)
  (Niagara|SpawnSystematLocation "/Game/MorphPond/Particles/PA_EnemyBlood.PA_EnemyBlood" (Transformation|GetActorLocation) "0, 0, 0" (* (Variables|Default|GetDefaultScale) "2.000000,2.000000,2.000000"))
  (CallFunction|Knockback (* Knockback%20Multiplier 1e+03) (* Knockback%20Multiplier 3e+02) Originator)
  (Rendering|Material|SetOverlayMaterial (Variables|Default|GetVisibleBody) "/Game/MorphPond/Materials/MA_WhiteFlash.MA_WhiteFlash" :!class /Script/Engine.MeshComponent)
  (Utilities|Time|SetTimerbyEvent (delegate Custom|Clear%20Overlay) 0.15)
  (Utilities|FlowControl|DelayUntilNextTick)
  (switch int (Variables|/Game/MorphPond/Characters/BP_CharacterBaseClass.BP_CharacterBaseClass_C|GetCountEnemiesBeingHit (Variables|Default|GetAttacker))
    (:Default
      (Class|FMODAudioComponent|SetEvent _fmod_hitbyplayerbite "/Game/FMOD/Events/BiteHitsEnemy_x3.BiteHitsEnemy_x3"))
    (:0
      (Class|FMODAudioComponent|SetEvent _fmod_hitbyplayerbite "/Game/FMOD/Events/BiteHitsEnemy.BiteHitsEnemy" :!label _label))
    (:1
      (goto _label))
    (:2
      (Class|FMODAudioComponent|SetEvent _fmod_hitbyplayerbite "/Game/FMOD/Events/BiteHitsEnemy_x2.BiteHitsEnemy_x2")))
  (CallFunction|HitstopsTakingDamage)
  (CallFunction|ChangeHealth (* Damage -1))
  (bind _alive (CallFunction|DeathCheck))
  (if _alive
    (Class|FMODAudioComponent|Play (Variables|Default|GetFMOD_HitByPlayerBite))
    (Components|Timeline|SetPlayRate (Variables|Default|GetTimeline_1a) 0.6)
    (bind _output_get (Variables|Default|SetBlipScale 5.0))
    (bind (_direction _blip _blipinverse) (Timeline|Timeline_1a PlayFromStart)
      (:Update
        (CallFunction|BlipUpdate _blip _blipinverse _visiblebody _output_get true false false))
      (:Finished
        (CallFunction|ResetScale _visiblebody))
      (:Halfway
        (Variables|Default|SetInvincibleToWeakAttacks false)
        (Variables|Default|SetAttacker 0)))
    (else
      (CallFunction|Death (Variables|Default|GetAttacker)))))

(event Custom|Spawn%20Collision
  (Game|SpawnActorfromClass "/Game/MorphPond/Engine/BP_BodyCollisionSphere.BP_BodyCollisionSphere_C" (Math|Transform|MakeTransform (Transformation|GetWorldLocation (Variables|Default|GetBodyContainer)) "0, 0, 0" (Variables|Default|GetDefaultScale)) "AlwaysSpawn" "MultiplyWithRoot" 0 (Variables|/Script/Engine.SphereComponent|GetSphereRadius (Variables|Default|GetBodyContainer)) self))

(event Custom|Death
  (params (Killer :type Actor%20Object%20Reference))
  (bind _deathhitstop (Variables|Default|GetDeathHitStop))
  ;[1 1 1] Death
  (Variables|Default|SetKiller Killer)
  (Camera|PlayWorldCameraShake "/Game/MorphPond/Camera/ScreenShake_Large.ScreenShake_Large_C" (Transformation|GetActorLocation) 0.0 5e+03)
  (Niagara|SpawnSystematLocation "/Game/MorphPond/Particles/PA_EnemyDeath.PA_EnemyDeath" (Transformation|GetActorLocation) "0, 0, 0" (* (Variables|Default|GetDefaultScale) "1.500000,1.500000,1.500000"))
  (CallFunction|SpawnPointSound "/Game/FMOD/Events/BiteHitsEnemy.BiteHitsEnemy" (Transformation|GetActorLocation) 0.0 "/Game/MorphPond/Camera/ScreenShake_Large.ScreenShake_Large_C")
  (bind _asbp_character_base_class (Utilities|Casting|CastToBP_CharacterBaseClass (Variables|Default|GetKiller)))
  (Rendering|Material|SetOverlayMaterial (Variables|Default|GetVisibleBody) "/Game/MorphPond/Materials/MA_White.MA_White" :!class /Script/Engine.MeshComponent)
  ;;[1 1 1] Hitstop on Self, Attacker, & UI
  (Default|StartHitstop _asbp_character_base_class _deathhitstop)
  (CallFunction|StartHitstop _deathhitstop)
  (if (Utilities|IsValid (Variables|/Game/MorphPond/Characters/BP_CharacterBaseClass.BP_CharacterBaseClass_C|GetActive%20Bite _asbp_character_base_class))
    (Default|StartHitstop (Variables|/Game/MorphPond/Characters/BP_CharacterBaseClass.BP_CharacterBaseClass_C|GetActive%20Bite _asbp_character_base_class) _deathhitstop))
  (Utilities|FlowControl|Delay 0.0)
  (CallFunction|SpawnPointSound "/Game/FMOD/Events/BiteHitsEnemy.BiteHitsEnemy" (Transformation|GetActorLocation) 0.35 "/Game/MorphPond/Camera/ScreenShake_Large2.ScreenShake_Large2_C")
  (bind _asbp_player_character (Utilities|Casting|CastToBP_PlayerCharacter (Variables|Default|GetKiller))
    (:then
      (Default|EnemyKilled _asbp_player_character (Variables|Default|GetFood))
      (Utilities|Casting|CastToBP_Fangs (Variables|Default|GetIncoming%20Attack)
        (:then
          (Default|ChangeStamina _asbp_player_character 3))
        (:CastFailed
          _)))
    (:CastFailed
      _))
  (Actor|DestroyActor))

(event Custom|Clear%20Overlay
  ;[1 1 1] Hit by Weak Attack
  (Rendering|Material|SetOverlayMaterial (Variables|Default|GetVisibleBody) 0 :!class /Script/Engine.MeshComponent))

(event Custom|AI%20Special%20Attack
  (CallFunction|CanSpecialAttack?)
  (switch int (.Value (Utilities|Map|Find (Variables|Default|GetAbilityMap) (Variables|Default|GetSpecial%20Ability)))
    (:1
      (CallFunction|TongueAttack))
    (:2
      (CallFunction|CannonballAttack))))

(event EventBeginPlay
  ;[1 1 1] BeginPlay Set Body Component
  (|CallParentFunction)
  (Variables|Default|SetVisibleBody (Variables|Default|GetSphere_0))
  (Variables|Default|SetUIColor "(R=0.228278,G=0.075406,B=0.312500,A=1.000000)")
  (Variables|/Script/Engine.CharacterMovementComponent|SetMaxWalkSpeed (Variables|Character|GetCharacterMovement) 4e+02)
  (Variables|Default|SetIsPlayer? false)
  ;[1 1 1] Add Aggro Function
  (bind _asbp_character_base_class (Utilities|Casting|CastToBP_CharacterBaseClass (Game|Player|GetPlayerPawn 0)))
  (Utilities|Array|Add (Variables|Default|GetAggroList) _asbp_character_base_class))

(event EventDestroyed
  (if (not (== (Variables|Default|GetSpecial%20Ability) ""))
    (bind _asbp_player_character (Utilities|Casting|CastToBP_PlayerCharacter (Variables|Default|GetKiller)))
    (Default|AbsorbAbility _asbp_player_character (Variables|Default|GetSpecial%20Ability))))

(event EventOnLanded
  (params (Hit :type Hit%20Result%20Structure%20%28by%20ref%29))
  ;[1 1 1] Land Anim
  (CallFunction|LandAction))

(fn ConstructionScript)

(fn DeathCheck
  (return (> (Variables|Default|GetHealth) 0)))

(fn HitstopsTakingDamage
  (bind _bitehitstoptime (Variables|Default|GetBiteHitstopTime))
  (bind _bitehitstoptime_2 (Variables|Default|GetBiteHitstopTime))
  (bind _incoming_attack (Variables|Default|GetIncoming%20Attack))
  (Default|StartHitstop (Variables|Default|GetAttacker) _bitehitstoptime_2)
  (CallFunction|StartHitstop _bitehitstoptime_2)
  (Utilities|IsValid _incoming_attack
    (:Is%20Valid
      (bind _asbp_2dattack_base_class (Utilities|Casting|CastToBP_2DAttackBaseClass _incoming_attack)
        (:then
          (Default|StartHitstop _asbp_2dattack_base_class _bitehitstoptime))
        (:CastFailed
          (bind _asbp_3dattack_base_class (Utilities|Casting|CastToBP_3DAttackBaseClass _incoming_attack))
          (Default|StartHitstop _asbp_3dattack_base_class _bitehitstoptime))))
    (:Is%20Not%20Valid
      _))
  (return))

(fn GetBestDirection
  (LocalVariables|SetMax -1e+02)
  (for (_array_element _array_index) (Variables|Default|GetDirectionWeights)
    (if (> _array_element (LocalVariables|GetMax))
      (LocalVariables|SetMax _array_element)
      (bind _output_get (LocalVariables|SetBest _array_index))))
  (return (Math|Vector|Normalize (+ (Transformation|GetActorLocation) (* (Utilities|Array|Get(acopy) (Variables|Default|GetMoveDirections) _output_get) "500.000000,500.000000,500.000000")))))