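; Player character, built on a parent character class, that bites, uses an absorbed special ability and spends food from kills to heal.
; Capsule overlaps with enemy bites and attack actors feed WeakAttack, which applies damage, brief invincibility, hitstop, camera shake, overlay flash and a timeline-driven squash-and-stretch.
; Health changes trigger engine pauses and hurt feedback, with death reloading the Test level.
; Tick takes spring arm height from a separate Z-lag component.
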(event OnComponentBeginOverlap(CapsuleComponent)
  (params (OverlappedComponent :type Primitive%20Component%20Object%20Reference) (OtherActor :type Actor%20Object%20Reference) (OtherComp :type Primitive%20Component%20Object%20Reference) (OtherBodyIndex :type Integer) (bFromSweep :type Boolean) (SweepResult :type Hit%20Result%20Structure%20%28by%20ref%29))
  ;[1 1 1] Hit by Bite
  ;;[1 1 1] Garbo
  (bind _asbp_enemy_character (Utilities|Casting|CastToBP_EnemyCharacter OtherActor)
    (:then
      (bind _output_get (Variables|Default|SetAttacker _asbp_enemy_character))
      (if (Math|Boolean|ANDBoolean (Variables|/Game/MorphPond/Characters/BP_CharacterBaseClass.BP_CharacterBaseClass_C|GetIsBiting? _asbp_enemy_character) (not (Variables|Default|GetInvincibleToWeakAttacks)) (Components|ComponentHasTag OtherComp "Bite"))
        (Variables|Default|SetIncomingDamage (Variables|/Game/MorphPond/Characters/BP_CharacterBaseClass.BP_CharacterBaseClass_C|GetBiteDamage _output_get))
        (CallFunction|WeakAttack (Variables|/Game/MorphPond/Characters/BP_CharacterBaseClass.BP_CharacterBaseClass_C|GetBiteDamage _output_get))))
    (:CastFailed
      (bind _asbp_3dattack_base_class (Utilities|Casting|CastToBP_3DAttackBaseClass OtherActor)
        (:then
          (bind _asbp_enemy_character_2 (Utilities|Casting|CastToBP_EnemyCharacter (Variables|/Script/Engine.Actor|GetInstigator _asbp_3dattack_base_class)))
          (Variables|Default|SetAttacker _asbp_enemy_character_2)
          (Utilities|IsValid _asbp_enemy_character_2
            (:Is%20Valid
              (if (and (Variables|/Game/MorphPond/Characters/BP_CharacterBaseClass.BP_CharacterBaseClass_C|GetIsSpecialAttacking? _asbp_enemy_character_2) (not (Variables|Default|GetInvincibleToWeakAttacks)))
                (Variables|Default|SetIncomingDamage (Variables|/Game/MorphPond/Attacks/BP_3DAttackBaseClass.BP_3DAttackBaseClass_C|GetDamage _asbp_3dattack_base_class))
                (CallFunction|WeakAttack (Variables|/Game/MorphPond/Attacks/BP_3DAttackBaseClass.BP_3DAttackBaseClass_C|GetDamage _asbp_3dattack_base_class))))))
        (:CastFailed
          (bind _asbp_2dattack_base_class (Utilities|Casting|CastToBP_2DAttackBaseClass OtherActor))
          (bind _asbp_enemy_character_3 (Utilities|Casting|CastToBP_EnemyCharacter (Variables|/Script/Engine.Actor|GetInstigator _asbp_2dattack_base_class)))
          (Variables|Default|SetAttacker _asbp_enemy_character_3)
          (Utilities|IsValid _asbp_enemy_character_3
            (:Is%20Valid
              (if (and (Variables|/Game/MorphPond/Characters/BP_CharacterBaseClass.BP_CharacterBaseClass_C|GetIsBiting? _asbp_enemy_character_3) (not (Variables|Default|GetInvincibleToWeakAttacks)))
                (bind _asbp_fangs (Utilities|Casting|CastToBP_Fangs OtherActor))
                (Variables|Default|SetIncomingDamage (Variables|/Game/MorphPond/Attacks/BP_2DAttackBaseClass.BP_2DAttackBaseClass_C|GetDamage _asbp_fangs))
                (CallFunction|WeakAttack (Variables|/Game/MorphPond/Attacks/BP_2DAttackBaseClass.BP_2DAttackBaseClass_C|GetDamage _asbp_fangs))))))))))

(event Custom|Weak%20Attack
  (params (Damage :type Integer%20%28by%20ref%29))
  (bind _attacker (Variables|Default|GetAttacker))
  (bind _attacker_2 (Variables|Default|GetAttacker))
  (bind _bitehitstoptime (Variables|Default|GetBiteHitstopTime))
  (bind _active_special_attack (Variables|/Game/MorphPond/Characters/BP_CharacterBaseClass.BP_CharacterBaseClass_C|GetActive%20Special%20Attack _attacker_2))
  (bind _active_bite (Variables|/Game/MorphPond/Characters/BP_CharacterBaseClass.BP_CharacterBaseClass_C|GetActive%20Bite _attacker_2))
  ;[1 1 1] Hit by Bite
  (Variables|Default|SetInvincibleToWeakAttacks true)
  (CallFunction|ChangeHealth (* (Variables|Default|GetIncomingDamage) -1))
  (Camera|PlayWorldCameraShake "/Game/MorphPond/Camera/ScreenShake_Large.ScreenShake_Large_C" (Transformation|GetActorLocation) 0.0 5e+03 1.0 true)
  (Niagara|SpawnSystematLocation "/Game/MorphPond/Particles/PA_PlayerBlood.PA_PlayerBlood" (Transformation|GetActorLocation) "0, 0, 0" "2.000000,2.000000,2.000000")
  (Rendering|Material|SetOverlayMaterial (Variables|Default|GetVisibleBody) "/Game/MorphPond/Materials/MA_White.MA_White" :!class /Script/Engine.MeshComponent)
  (Utilities|Time|SetTimerbyEvent (delegate Custom|Clear%20Overlay) (Variables|Default|GetBiteHitstopTime))
  (Utilities|IsValid _attacker
    (:Is%20Valid
      (Default|StartHitstop _attacker _bitehitstoptime))
    (:Is%20Not%20Valid
      _))
  (CallFunction|StartHitstop _bitehitstoptime)
  (Utilities|IsValid _active_bite
    (:Is%20Valid
      (Default|StartHitstop _active_bite 0.05))
    (:Is%20Not%20Valid
      _))
  (Utilities|IsValid _active_special_attack
    (:Is%20Valid
      (Default|StartHitstop _active_special_attack 0.05))
    (:Is%20Not%20Valid
      _))
  (Components|Timeline|SetPlayRate (Variables|Default|GetTimeline_1_0) 0.6)
  (Variables|Default|SetBlipScale 5.0)
  (bind (_direction _blip _blipinverse) (Timeline|Timeline_1_0 PlayFromStart)
    (:Update
      (Utilities|Blip _blip (Variables|Default|GetVisibleBody) _blipinverse :!label _label))
    (:Finished
      (goto _label finished))
    (:Halfway
      (Rendering|Material|SetOverlayMaterial (Variables|Default|GetVisibleBody) 0 :!class /Script/Engine.MeshComponent)
      (Utilities|FlowControl|Delay 0.8)
      (Variables|Default|SetInvincibleToWeakAttacks false))))

(event Custom|Clear%20Overlay
  ;[1 1 1] Hit by Bite
  (Rendering|Material|SetOverlayMaterial (Variables|Default|GetVisibleBody) "/Game/MorphPond/Materials/MA_Red.MA_Red" :!class /Script/Engine.MeshComponent))

(event Custom|Absorb%20Ability
  (params (Ability :type Name))
  ;[1 1 1] Absorb Ability
  (Niagara|SpawnSystematLocation "/Game/MorphPond/Particles/PA_AbsorbAbility.PA_AbsorbAbility" (Transformation|GetActorLocation) "0, 0, 0" "1.500000,1.500000,1.500000")
  (CallFunction|ChangeHealth 2)
  (Default|PauseforTime (Variables|Default|GetEngineReference) 1.0)
  (Utilities|FlowControl|Delay 1.0)
  (bind _output_get (Variables|Default|SetSpecial%20Ability Ability))
  (switch int (.Value (Utilities|Map|Find (Variables|Default|GetAbilityMap) _output_get))
    (:1
      (CallFunction|TongueAbsorbAnim))
    (:2
      (CallFunction|CannonballAbsorbAnim)))
  (Default|PauseforTime (Variables|Default|GetEngineReference) 1.0))

(event Custom|Enemy%20Killed
  (params (Food%20Gained :type Integer))
  (CallFunction|ChangeFood Food%20Gained 0.0)
  (CallFunction|UpdateFoodHUD 0.42))

(event Custom|Update%20Food%20HUD
  (params (Visual%20Delay :type Float%20%28double-precision%29))
  (bind _asbp_player_controller (Utilities|Casting|CastToBP_PlayerController (Pawn|GetController)))
  (Default|ChangeFood (Variables|/Game/MorphPond/Characters/BP_PlayerController.BP_PlayerController_C|GetHUD _asbp_player_controller) (Variables|Default|GetFood) Visual%20Delay)
  (Utilities|FlowControl|Delay Visual%20Delay)
  (Class|FMODAudioComponent|Play (Variables|Default|GetFMOD_Food)))

(event Custom|Death
  (Rendering|SetVisibility (Variables|Default|GetVisibleBody) false true)
  (Camera|PlayWorldCameraShake "/Game/MorphPond/Camera/ScreenShake_Large.ScreenShake_Large_C" (Transformation|GetActorLocation) 0.0 5e+03)
  (Niagara|SpawnSystematLocation "/Game/MorphPond/Particles/PA_EnemyDeath.PA_EnemyDeath" (Transformation|GetActorLocation) "0, 0, 0" "3.000000,3.000000,3.000000")
  (Utilities|FlowControl|Delay 2.0)
  (Game|OpenLevel(byName) "Test"))

(event Input|EnhancedActionEvents|EnhancedInputActionIA_SecondaryRelease
  (params (ActionValue :type Boolean) (ElapsedSeconds :type Float%20%28double-precision%29) (TriggeredSeconds :type Float%20%28double-precision%29) (InputAction :type Input%20Action%20Object%20Reference :default "/Game/MorphPond/Controls/IA_SecondaryRelease.IA_SecondaryRelease"))
  (:Triggered
    (CallFunction|SpecialReleased)))

(event Input|EnhancedActionEvents|EnhancedInputActionIA_Attack
  (params (ActionValue :type Boolean) (ElapsedSeconds :type Float%20%28double-precision%29) (TriggeredSeconds :type Float%20%28double-precision%29) (InputAction :type Input%20Action%20Object%20Reference :default "/Game/MorphPond/Controls/IA_Attack.IA_Attack"))
  ;[1 1 1] Bite Attack
  (:Started
    (CallFunction|BiteAttackAction)))

(event Input|EnhancedActionEvents|EnhancedInputActionIA_AttackHold
  (params (ActionValue :type Boolean) (ElapsedSeconds :type Float%20%28double-precision%29) (TriggeredSeconds :type Float%20%28double-precision%29) (InputAction :type Input%20Action%20Object%20Reference :default "/Game/MorphPond/Controls/IA_AttackHold.IA_AttackHold"))
  (:Triggered
    (CallFunction|BiteHoldAttackAction))
  (:Completed
    (CallFunction|BiteHoldReleaseAction)))

(event Input|EnhancedActionEvents|EnhancedInputActionIA_HoldSpecialHeal
  (params (ActionValue :type Boolean) (ElapsedSeconds :type Float%20%28double-precision%29) (TriggeredSeconds :type Float%20%28double-precision%29) (InputAction :type Input%20Action%20Object%20Reference :default "/Game/MorphPond/Controls/IA_HoldSpecialHeal.IA_HoldSpecialHeal"))
  (:Triggered
    (Utilities|Casting|CastToBP_PlayerController (Game|GetPlayerController 0))
    (if (and (not (Variables|Default|GetIsWalking?)) (> (Variables|Default|GetFood) 0))
      (CallFunction|ChangeHealth 1)
      (CallFunction|ChangeFood -1 0.0)
      (Camera|PlayWorldCameraShake "/Game/MorphPond/Camera/ScreenShake_Mid.ScreenShake_Mid_C" (Transformation|GetActorLocation) 0.0 1e+03 1.0 true)
      (Rendering|Material|SetOverlayMaterial (Variables|Default|GetVisibleBody) "/Game/MorphPond/Materials/MA_PulseColour.MA_PulseColour" :!class /Script/Engine.MeshComponent)
      (CallFunction|ChargeAnim 1.0 4.0 true false false)
      (Utilities|FlowControl|Delay 0.3)
      (Rendering|Material|SetOverlayMaterial (Variables|Default|GetVisibleBody) 0 :!class /Script/Engine.MeshComponent))))

(event EventBeginPlay
  ;[1 1 1] BeginPlay
  (|CallParentFunction)
  (Variables|Default|SetIsPlayer? true)
  (bind _outactors (Actor|GetAllActorsOfClass "/Game/MorphPond/Engine/BP_Engine.BP_Engine_C"))
  (for _array_element _outactors
    (Variables|Default|SetEngineReference _array_element))
  (CallFunction|Initialise)
  (Variables|Default|SetSpecial%20Ability "None")
  (Variables|Default|SetBodyType "Water"))

(event EventChangeHealth
  (params (Amount :type Integer))
  (|CallParentFunction Amount)
  (if (< Amount 0)
    (Components|Activation|Activate (Variables|Default|GetPA_PlayerDamageOverlay) false)
    (Class|FMODAudioComponent|Play (Variables|Default|GetFMOD_Hurt))
    (Default|PauseforTime (Variables|Default|GetEngineReference) 0.75)
    (if (<= (Variables|Default|GetHealth) 0)
      (CallFunction|Death))))

(event EventOnLanded
  (params (Hit :type Hit%20Result%20Structure%20%28by%20ref%29))
  ;[1 1 1] Land Anim
  (CallFunction|LandAction))

(event EventTick
  (params (DeltaSeconds :type Float%20%28single-precision%29))
  (bind _springarm (Variables|Default|GetSpringArm))
  (bind _returnvalue (Transformation|GetWorldLocation _springarm))
  (|CallParentFunction 0.0)
  (Transformation|SetWorldLocation _springarm (Math|Vector|MakeVector (.x _returnvalue) (.y _returnvalue) (.z (Transformation|GetWorldLocation (Variables|Default|GetSpringArmZLag)))) false false))

(fn ConstructionScript)

(fn Initialise
  (Variables|Default|SetVisibleBody (Variables|Default|GetSphere_0))
  (Variables|Default|SetUIColor "(R=0.546875,G=0.076429,B=0.038311,A=1.000000)")
  (bind _output_get (Variables|Default|SetMaxHealth 5))
  (bind _output_get_2 (Variables|Default|SetHealth _output_get))
  (bind _output_get_3 (Variables|Default|SetMaxStamina _output_get_2))
  (Variables|Default|SetStamina _output_get_3)
  (Variables|Default|SetDefaultScale "1.000000,1.000000,1.000000")
  (Variables|Default|SetSpecial%20Ability "None"))