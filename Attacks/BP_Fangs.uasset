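; BP_Fangs is a character bite attack: a projectile sprite tinted with the instigator's UIColor, animated by timeline-driven scale "blips".
; Bite plays the blip over a short lifespan based on AnimationSpeed.
; BiteHold halts movement, attaches to the instigator with a long lifespan, and Tick reduces blip strength while it is held and the character is biting.
; Construction caches the instigator's default scale and sets projectile speed; destruction clears the instigator's ActiveBite.
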(event Custom|Bite
  (bind _rendercomponent (Variables|Default|GetRenderComponent))
  ;[1 1 1] Bite
  (Actor|SetLifeSpan (* (Variables|Default|GetAnimation%20Speed) 0.2))
  (bind _asbp_character_base_class (Utilities|Casting|CastToBP_CharacterBaseClass (Variables|Default|GetInstigator)))
  (Sprite|SetSpriteColor (Variables|Default|GetRenderComponent) (Variables|/Game/MorphPond/Characters/BP_CharacterBaseClass.BP_CharacterBaseClass_C|GetUIColor _asbp_character_base_class))
  (Components|Timeline|SetPlayRate (Variables|Default|GetTimeline) (/ 0.8 1.0))
  (Variables|Default|SetBlip%20Scale 2.5)
  (bind (_direction _blip _blipinverse _scale) (Timeline|Timeline Play)
    (:Update
      (Transformation|SetRelativeScale3D _rendercomponent (Math|Vector|MakeVector (.ReturnValue (Utilities|BlipScale _blip _blipinverse _scale _scale)) (.ReturnValue (Utilities|BlipScale _blip _blipinverse _scale _scale)) (.ReturnValue2 (Utilities|BlipScale _blip _blipinverse _scale _scale)))))
    (:Finished
      (Transformation|SetRelativeScale3D _rendercomponent (* (Variables|Default|GetScale) (Math|Vector|MakeVector 0.7 0.7 0.7))))))

(event Custom|BiteHold
  (bind _projectilemovement (Variables|Default|GetProjectileMovement))
  (bind _rendercomponent (Variables|Default|GetRenderComponent))
  ;[1 1 1] Bite Hold
  (Variables|/Script/Engine.MovementComponent|SetVelocity _projectilemovement "0.000000,-0.600000,0.000000")
  (Variables|/Script/Engine.ProjectileMovementComponent|SetMaxSpeed _projectilemovement 0.0)
  (Actor|SetLifeSpan 3e+01)
  (bind _asbp_character_base_class (Utilities|Casting|CastToBP_CharacterBaseClass (Variables|Default|GetInstigator)))
  (Sprite|SetSpriteColor (Variables|Default|GetRenderComponent) (Variables|/Game/MorphPond/Characters/BP_CharacterBaseClass.BP_CharacterBaseClass_C|GetUIColor _asbp_character_base_class))
  (Components|Timeline|SetPlayRate (Variables|Default|GetTimeline_1) (/ 0.8 1.0))
  (Variables|Default|SetBlip%20Scale 2.6)
  (Variables|Default|SetIsHeld true)
  (bind _asbp_character_base_class_2 (Utilities|Casting|CastToBP_CharacterBaseClass (Variables|Default|GetInstigator)))
  (Transformation|SetActorLocation (Transformation|GetWorldLocation (Variables|/Script/Engine.Character|GetCapsuleComponent _asbp_character_base_class_2)) false false)
  (Transformation|AttachActorToActor _asbp_character_base_class_2 "None" "SnapToTarget" "KeepRelative" "SnapToTarget" true)
  (bind (_direction _blip _blipinverse _scale) (Timeline|Timeline_1 PlayFromStart)
    (:Update
      (Transformation|SetRelativeScale3D _rendercomponent (Math|Vector|MakeVector (.ReturnValue (Utilities|BlipScale1 _blip _blipinverse _scale _scale)) (.ReturnValue (Utilities|BlipScale1 _blip _blipinverse _scale _scale)) (.ReturnValue2 (Utilities|BlipScale1 _blip _blipinverse _scale _scale)))))
    (:Finished
      (Transformation|SetRelativeScale3D _rendercomponent (Math|Vector|MakeVector (.ReturnValue (Utilities|BlipScale1 _blip _blipinverse _scale _scale)) (.ReturnValue (Utilities|BlipScale1 _blip _blipinverse _scale _scale)) (.ReturnValue2 (Utilities|BlipScale1 _blip _blipinverse _scale _scale)))))))

(event EventBeginPlay
  ;[1 1 1] Begin Play
)

(event EventTick
  (params (DeltaSeconds :type Float%20%28single-precision%29))
  (if (Utilities|IsValid (Variables|Default|GetAs%20BP%20Character%20Base%20Class))
    (if (and (Variables|/Game/MorphPond/Characters/BP_CharacterBaseClass.BP_CharacterBaseClass_C|GetIsBiting? (Variables|Default|GetAs%20BP%20Character%20Base%20Class)) (Variables|Default|GetIsHeld))
      (Variables|Default|SetBlip%20Scale 0.3)
      (Components|Timeline|SetPlayRate (Variables|Default|GetTimeline_0) (/ 0.8 1.0)))))

(event EventDestroyed
  (bind _instigator (Variables|Default|GetInstigator))
  ;[1 1 1] Destroyed
  (if (Utilities|IsValid _instigator)
    (bind _asbp_character_base_class (Utilities|Casting|CastToBP_CharacterBaseClass _instigator))
    (Variables|/Game/MorphPond/Characters/BP_CharacterBaseClass.BP_CharacterBaseClass_C|SetActive%20Bite _asbp_character_base_class 0)))

(fn ConstructionScript
  (bind _projectilemovement (Variables|Default|GetProjectileMovement))
  (bind _asbp_character_base_class (Utilities|Casting|CastToBP_CharacterBaseClass (Variables|Default|GetInstigator)))
  (bind _output_get (Variables|Default|SetAs%20BP%20Character%20Base%20Class _asbp_character_base_class))
  (bind _output_get_2 (Variables|Default|SetDefault%20Scale%20Vect (Variables|/Game/MorphPond/Characters/BP_CharacterBaseClass.BP_CharacterBaseClass_C|GetDefaultScale _output_get)))
  (Variables|Default|SetDefault%20Scale%20Float (.x _output_get_2))
  (bind _output_get_3 (Variables|/Script/Engine.ProjectileMovementComponent|SetMaxSpeed _projectilemovement (Variables|Default|GetSpeed)))
  (Variables|/Script/Engine.ProjectileMovementComponent|SetInitialSpeed _projectilemovement _output_get_3))