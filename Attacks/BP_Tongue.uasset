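; BP_Tongue is a tongue attack projectile that launches out and returns to the character that fired it.
; Shortly after spawn, timers enable homing on HomingTargetComponent, then set the homing acceleration.
; Each tick it matches the Instigator's height and shrinks its sphere with horizontal distance from them.
; Once homing and near the Instigator it calls TongueReturn and destroys itself, also expiring on lifespan or an invalid Instigator.
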(event Custom|Return
  (Variables|/Script/Engine.ProjectileMovementComponent|SetbIsHomingProjectile (Variables|Default|GetProjectileMovement) true)
  (Variables|/Script/Engine.ProjectileMovementComponent|SetHomingTargetComponent (Variables|Default|GetProjectileMovement) (Variables|Default|GetHoming%20Target%20Component)))

(event Custom|Speed%20Up
  (Variables|/Script/Engine.ProjectileMovementComponent|SetHomingAccelerationMagnitude (Variables|Default|GetProjectileMovement) 6e+04))

(event EventBeginPlay
  (Variables|Default|SetInitialVelocity (Variables|/Script/Engine.MovementComponent|GetVelocity (Variables|Default|GetProjectileMovement)))
  (Actor|SetLifeSpan 2.0)
  (Utilities|Time|SetTimerbyEvent (delegate Custom|Return) 0.1)
  (Utilities|Time|SetTimerbyEvent (delegate Custom|Speed%20Up) 0.7))

(event EventTick
  (params (DeltaSeconds :type Float%20%28single-precision%29))
  (bind _returnvalue (Transformation|GetActorLocation))
  (bind _instigator (Variables|Default|GetInstigator))
  (bind _returnvalue_2 (Transformation|GetHorizontalDistanceTo _instigator))
  (Utilities|IsValid (Variables|Default|GetInstigator)
    (:Is%20Valid
      (Transformation|SetActorLocation (Math|Vector|MakeVector (.x _returnvalue) (.y _returnvalue) (.z (Transformation|GetActorLocation (Variables|Default|GetInstigator)))) true false)
      (Transformation|SetRelativeScale3D (Variables|Default|GetSphere1) (* (/ 3.0 (Math|Float|MapRangeClamped _returnvalue_2 1e+02 2e+03 1.0 5.0)) (Math|Vector|MakeVector 1.0 1.0 1.0)))
      (if (and (<= _returnvalue_2 2e+02) (Variables|/Script/Engine.ProjectileMovementComponent|GetbIsHomingProjectile (Variables|Default|GetProjectileMovement)))
        (bind _asbp_character_base_class (Utilities|Casting|CastToBP_CharacterBaseClass (Variables|Default|GetInstigator)))
        (Default|TongueReturn _asbp_character_base_class)
        (Actor|DestroyActor)))
    (:Is%20Not%20Valid
      (Actor|DestroyActor))))

(event EventDestroyed)

(fn ConstructionScript
  (|CallParentFunction))