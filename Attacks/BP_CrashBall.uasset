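; BP_CrashBall is an attack actor that stays attached by position to the character or actor that instigated it.
; Each Tick, after the parent Tick runs, it moves to the Instigator's location with a swept move, and destroys itself if the Instigator is no longer valid.
; It adds no overlap or construction logic of its own.
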(event EventBeginPlay
  (|CallParentFunction) ; This node is disabled and will not be called.\nDrag off pins to build functionality.
)

(event Collision|EventActorBeginOverlap
  (params (OtherActor :type Actor%20Object%20Reference))
  (|CallParentFunction OtherActor) ; This node is disabled and will not be called.\nDrag off pins to build functionality.
)

(event EventTick
  (params (DeltaSeconds :type Float%20%28single-precision%29))
  (bind _instigator (Variables|Default|GetInstigator))
  (bind _returnvalue (Transformation|GetActorLocation _instigator))
  (|CallParentFunction DeltaSeconds)
  (Utilities|IsValid (Variables|Default|GetInstigator)
    (:Is%20Valid
      (Transformation|SetActorLocation (Math|Vector|MakeVector (.x _returnvalue) (.y _returnvalue) (.z _returnvalue)) true false))
    (:Is%20Not%20Valid
      (Actor|DestroyActor))))

(fn ConstructionScript
  (|CallParentFunction))