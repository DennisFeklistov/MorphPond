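; BP_FlingJelly is a pulsing jelly attack actor with a sphere and cable that reacts to its distance from its Instigator.
; A self-restarting Timeline feeds curve and inverse curve into BlipUpdate, squash-and-stretching the sphere around its spawn scale.
; Tick resizes Sphere1 and switches between calm purple jelly and a faster, stronger flaming pulse once far enough away horizontally.
; The actor destroys itself when the Instigator becomes invalid.
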(event Custom|Restart%20Anim
  (bind (_direction _blip _blipinverse) (Timeline|Timeline PlayFromStart)
    (:Update
      (CallFunction|BlipUpdate _blip _blipinverse (Variables|Default|GetSphere) (Variables|Default|GetAnim%20Rate) true false false))
    (:Finished
      (CallFunction|RestartAnim))))

(event EventBeginPlay
  (Variables|Default|SetDefault%20Scale (Transformation|GetActorScale3D))
  (bind (_direction _blip _blipinverse) (Timeline|Timeline PlayFromStart)
    (:Update
      (CallFunction|BlipUpdate _blip _blipinverse (Variables|Default|GetSphere) (Variables|Default|GetAnim%20Rate) true false false))
    (:Finished
      (CallFunction|RestartAnim))))

(event Collision|EventActorBeginOverlap
  (params (OtherActor :type Actor%20Object%20Reference)))

(event EventTick
  (params (DeltaSeconds :type Float%20%28single-precision%29))
  (bind _instigator (Variables|Actor|GetInstigator))
  (bind _returnvalue (Transformation|GetHorizontalDistanceTo _instigator))
  (Utilities|IsValid (Variables|Actor|GetInstigator)
    (:Is%20Valid
      (if (>= _returnvalue 3e+02)
        (Transformation|SetRelativeScale3D (Variables|Default|GetSphere1) (* (/ 3.0 2.0) (Math|Vector|MakeVector 1.0 1.0 1.0)))
        (bind _output_get (Variables|Default|SetAnim%20Rate 6.0))
        (Components|Timeline|SetPlayRate (Variables|Default|GetTimeline) (/ _output_get 3.0))
        (Rendering|Material|SetOverlayMaterial (Variables|Default|GetSphere) "/Game/MorphPond/Materials/M_Flame.M_Flame" :!class /Script/Engine.MeshComponent)
        (Rendering|Material|SetMaterial (Variables|Default|GetSphere) 0 "/Game/MorphPond/Materials/MA_PulseColour.MA_PulseColour")
        (Rendering|Material|SetMaterial (Variables|Default|GetCable) 0 "/Game/MorphPond/Materials/M_Flame.M_Flame")
        (else
          (Transformation|SetRelativeScale3D (Variables|Default|GetSphere1) (* (/ 3.0 (Math|Float|MapRangeClamped _returnvalue 1e+02 2e+03 1.0 5.0)) (Math|Vector|MakeVector 1.0 1.0 1.0)))
          (bind _output_get_2 (Variables|Default|SetAnim%20Rate 1.0))
          (Components|Timeline|SetPlayRate (Variables|Default|GetTimeline) (/ _output_get_2 3.0))
          (Rendering|Material|SetOverlayMaterial (Variables|Default|GetSphere) "/Game/MorphPond/Materials/M_Jelly.M_Jelly" :!class /Script/Engine.MeshComponent)
          (Rendering|Material|SetMaterial (Variables|Default|GetSphere) 0 "/Game/MorphPond/Materials/Pallete1/MA_PurpleJelly.MA_PurpleJelly")
          (Rendering|Material|SetMaterial (Variables|Default|GetCable) 0 "/Game/MorphPond/Materials/M_Jelly.M_Jelly"))))
    (:Is%20Not%20Valid
      (Actor|DestroyActor))))

(fn ConstructionScript)

(fn BlipUpdate
  (params (Curve :type Float%20%28double-precision%29) (CurveInverse :type Float%20%28double-precision%29) (Target :type Scene%20Component%20Object%20Reference) (Scale :type Float%20%28double-precision%29) (ScaleHeight? :type Boolean) (ScaleWidth? :type Boolean) (ScaleLength? :type Boolean))
  (bind _returnvalue (* Curve Scale))
  (bind _returnvalue_2 (* CurveInverse Scale))
  (bind _default_scale (Variables|Default|GetDefault%20Scale))
  (bind _returnvalue_3 (+ _returnvalue_2 1.0))
  (bind _returnvalue_4 (+ _returnvalue 1.0))
  (bind _returnvalue_5 (* _returnvalue_3 (.x _default_scale)))
  (bind _returnvalue_6 (* _returnvalue_4 (.x _default_scale)))
  (if ScaleHeight?
    (Transformation|SetWorldScale3D Target (Math|Vector|MakeVector _returnvalue_5 _returnvalue_5 _returnvalue_6))
    (elif ScaleWidth?
      (Transformation|SetWorldScale3D Target (Math|Vector|MakeVector _returnvalue_5 _returnvalue_6 _returnvalue_5))
      (else
        (Transformation|SetWorldScale3D Target (Math|Vector|MakeVector _returnvalue_6 _returnvalue_5 _returnvalue_5)))))
  (return))